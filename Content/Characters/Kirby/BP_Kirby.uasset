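; BP_Kirby is a playable character with camera look, movement, jump, sprint and crouch.
; Tick turns forward and strafe axes into movement relative to actor facing, while sprint doubles walk speed.
; Scroll feeds a clamped math expression that sets camera boom length, snapping to zero near the minimum for a close-in view.
; Crouch fakes a pose by squashing the mesh vertically and lowering the camera socket offset.
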(event EventTick
  (params (DeltaSeconds :type Float%20%28single-precision%29))
  (Pawn|Input|AddMovementInput (+ (* (Transformation|GetActorForwardVector) (Input|AxisValues|GetMovement_ForwardBack)) (* (Transformation|GetActorRightVector) (Input|AxisValues|GetMovement_Strafe))) 1.0 false))

(event Input|ActionEvents|InputActionMovement_Jump
  (params (Key :type Key%20Structure :default "AnyKey"))
  (:Pressed
    (Character|Jump)))

(event Input|ActionEvents|InputActionMovement_Sprint
  (params (Key :type Key%20Structure :default "AnyKey"))
  (bind _charactermovement (Variables|Character|GetCharacterMovement))
  (:Pressed
    (Variables|/Script/Engine.CharacterMovementComponent|SetMaxWalkSpeed _charactermovement 1.2e+03))
  (:Released
    (Variables|/Script/Engine.CharacterMovementComponent|SetMaxWalkSpeed _charactermovement 6e+02)))

(event Input|ActionEvents|InputActionMovement_Crouch
  (params (Key :type Key%20Structure :default "AnyKey"))
  (:Pressed
    (Character|Crouch)
    (Transformation|SetWorldScale3D (Variables|Character|GetMesh) "1.000000,1.000000,0.800000")
    (Variables|/Script/Engine.SpringArmComponent|SetSocketOffset (Variables|Components|GetCameraJig) "0, 0,32.000000"))
  (:Released
    (Character|UnCrouch)
    (Transformation|SetWorldScale3D (Variables|Character|GetMesh) "1.000000,1.000000,1.000000")
    (Variables|/Script/Engine.SpringArmComponent|SetSocketOffset (Variables|Components|GetCameraJig) "0, 0,64.000000")))

(event Input|AxisEvents|InputAxisView_Pitch
  (params (AxisValue :type Float%20%28single-precision%29))
  (Pawn|Input|AddControllerPitchInput AxisValue))

(event Input|AxisEvents|InputAxisView_Scroll
  (params (AxisValue :type Float%20%28single-precision%29))
  (bind _output_get (Variables|Default|SetGetJiggyWithIt (|(clamp(((A*25)+B),175,500)) AxisValue (Variables|Default|GetGetJiggyWithIt))))
  (Variables|/Script/Engine.SpringArmComponent|SetTargetArmLength (Variables|Components|GetCameraJig) (Math|Float|SelectFloat _output_get 0.0 (> (|(clamp(((A*25)+B),175,500)) AxisValue (Variables|Default|GetGetJiggyWithIt)) 2e+02))))

(event Input|AxisEvents|InputAxisView_Yaw
  (params (AxisValue :type Float%20%28single-precision%29))
  (Pawn|Input|AddControllerYawInput AxisValue))

(fn ConstructionScript)